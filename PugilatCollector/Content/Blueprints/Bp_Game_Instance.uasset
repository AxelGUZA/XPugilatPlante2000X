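; Game Instance that holds shared match state for a two-player game.
; On Init it resets each player's life, strength, power and selection, along with a global match timer and in-game and victory flags.
; It only sets these defaults; no logic here updates them, and Shutdown is empty.
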(event EventInit
  (Variables|Default|SetJ1_Life 1e+02)
  (Variables|Default|SetJ2_Life 1e+02)
  (Variables|Default|SetJ1_Strengh 1e+02)
  (Variables|Default|SetJ2_Strengh 1e+02)
  (Variables|Default|SetGlobal_Game_Chrono 120)
  (Variables|Default|SetJ1_Selection 0)
  (Variables|Default|SetJ2_Selection 0)
  (Variables|Default|SetIsInGame false)
  (Variables|Default|SetIsVictoire false)
  (Variables|Default|SetJ1_Power 0.0)
  (Variables|Default|SetJ2_Power 0.0))

(event EventShutdown)